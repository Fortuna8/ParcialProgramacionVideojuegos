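; BP_Personaje is an archer character that moves itself and can spawn BP_Dardo darts at its location.
; Tick offsets it by velocity times an acceleration factor, without delta time or sweep, while the construction script tints three meshes through dynamic materials.
; Functions double that factor or reverse X velocity, zeroing Y and Z.
; The enemy-relative aiming logic in DireccionarNormalizarFlecha never runs.
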(event EventTick
  (params (DeltaSeconds :type Float%20%28single-precision%29))
  (Transformation|AddActorWorldOffset (* (Variables|Default|GetVelocidad) (Variables|Default|GetaceleracionPersonaje))))

(fn ConstructionScript
  (bind _returnvalue (Rendering|Material|CreateDynamicMaterialInstance (Variables|Default|GetCylinder1) 0 0 "None" :!class /Script/Engine.PrimitiveComponent))
  (bind _returnvalue_2 (Rendering|Material|CreateDynamicMaterialInstance (Variables|Default|GetCylin1) 0 0 "None" :!class /Script/Engine.PrimitiveComponent))
  (bind _returnvalue_3 (Rendering|Material|CreateDynamicMaterialInstance (Variables|Default|GetSphere) 0 0 "None" :!class /Script/Engine.PrimitiveComponent))
  (Rendering|Material|SetVectorParameterValue _returnvalue "colorArquero" (Variables|Default|GetcolorPersonaje) :!class /Script/Engine.MaterialInstanceDynamic))

(fn SpawnearD
  (params (velocidad :type Vector) (orientation :type Rotator))
  (Game|SpawnActorfromClass "/Game/Blueprints/Ejercicio2/BP_Dardo.BP_Dardo_C" (Math|Transform|MakeTransform (Transformation|GetActorLocation) orientation "3.500000,3.500000,3.500000") "Undefined" "MultiplyWithRoot" 0 velocidad 0))

(fn SetAceleracionPersonaje
  (Variables|Default|SetaceleracionPersonaje (* (Variables|Default|GetaceleracionPersonaje) 2.0)))

(fn RevertirVelocidadPersonaje
  (Variables|Default|Setvelocidad (* (Variables|Default|Getvelocidad) "-1.000000,0.000000,0.000000")))