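; BP_Enemigo is an enemy actor that moves along a velocity vector and can fire darts.
; Tick offsets it by Velocidad times AceleracionEnemigo, without sweep or delta-time scaling, and SetVelocidadEnemigo sets that velocity.
; The construction script creates dynamic materials on its two cylinders and sphere, tinting them with ColorEnemigo through the colorOrco parameter.
; SpawnearDardoE spawns an enlarged BP_Dardo at its location with a given orientation and velocity.
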(event EventTick
  (params (DeltaSeconds :type Float%20%28single-precision%29))
  (Transformation|AddActorWorldOffset (* (Variables|Default|GetVelocidad) (Variables|Default|GetaceleracionEnemigo))))

(fn ConstructionScript
  (bind _returnvalue (Rendering|Material|CreateDynamicMaterialInstance (Variables|Default|GetCylinder1) 0 0 "None" :!class /Script/Engine.PrimitiveComponent))
  (bind _returnvalue_2 (Rendering|Material|CreateDynamicMaterialInstance (Variables|Default|GetCylinder) 0 "/Game/Blueprints/Ejercicio2/EnemigoSkinMaterial.EnemigoSkinMaterial" "None" :!class /Script/Engine.PrimitiveComponent))
  (bind _returnvalue_3 (Rendering|Material|CreateDynamicMaterialInstance (Variables|Default|GetSphere) 0 0 "None" :!class /Script/Engine.PrimitiveComponent))
  (Rendering|Material|SetVectorParameterValue _returnvalue "colorOrco" (Variables|Default|GetcolorEnemigo) :!class /Script/Engine.MaterialInstanceDynamic))

(fn SetVelocidadEnemigo
  (params (Velocidad :type Vector))
  (Variables|Default|SetVelocidad Velocidad))

(fn SpawnearDardoE
  (params (velocidad :type Vector) (orientation :type Rotator))
  (Game|SpawnActorfromClass "/Game/Blueprints/Ejercicio2/BP_Dardo.BP_Dardo_C" (Math|Transform|MakeTransform (Transformation|GetActorLocation) orientation "3.500000,3.500000,3.500000") "Undefined" "MultiplyWithRoot" 0 velocidad 0))