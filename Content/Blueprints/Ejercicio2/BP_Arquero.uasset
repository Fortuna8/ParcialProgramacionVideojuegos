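; BP_Arquero is an archer actor that can spawn BP_Flecha arrows with a given velocity and orientation.
; Its Construction Script tints three meshes through dynamic materials using ColorArquero, and BeginPlay draws a long-lived debug box around it.
; SpawnearFlechas spawns enlarged arrows at the actor's location but has no caller here.
; An unconnected graph, DireccionarNormalizarFlecha, computes a normalized orc-to-archer vector scaled by VelocidadFlecha.
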(event EventBeginPlay
  (Rendering|Debug|DrawDebugBox (Transformation|GetActorLocation) "50.000000,50.000000,50.000000" "(R=0.196835,G=1.000000,B=0.248990,A=1.000000)" "0, 0, 0" 3.6e+03 1e+01))

(fn ConstructionScript
  (bind _returnvalue (Rendering|Material|CreateDynamicMaterialInstance (Variables|Default|GetCylinder1) 0 0 "None" :!class /Script/Engine.PrimitiveComponent))
  (bind _returnvalue_2 (Rendering|Material|CreateDynamicMaterialInstance (Variables|Default|GetCylin1) 0 0 "None" :!class /Script/Engine.PrimitiveComponent))
  (bind _returnvalue_3 (Rendering|Material|CreateDynamicMaterialInstance (Variables|Default|GetSphere) 0 0 "None" :!class /Script/Engine.PrimitiveComponent))
  (Rendering|Material|SetVectorParameterValue _returnvalue "colorArquero" (Variables|Default|GetcolorArquero) :!class /Script/Engine.MaterialInstanceDynamic))

(fn SpawnearFlechas
  (params (velocidad :type Vector) (orientation :type Rotator))
  (Game|SpawnActorfromClass "/Game/Blueprints/Ejercicio2/BP_Flecha.BP_Flecha_C" (Math|Transform|MakeTransform (Transformation|GetActorLocation) orientation "3.500000,3.500000,3.500000") "Undefined" "MultiplyWithRoot" 0 velocidad 0))